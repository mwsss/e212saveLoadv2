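; BP_ch01 is an input-handling Blueprint that runs a one-second counter and toggles the WG_m01 widget.
; BeginPlay creates the widget hidden, then loops through a Delay that increments NTime and writes it to a TextRender.
; Q or the flipVw event drives a shared FlipFlop that switches widget visibility and mouse cursor display.
; E resets the counter to zero.
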(event `self.ReceiveBeginPlay`
  (bind _returnvalue (`|CreateWidget` "/Game/HUD/WG_m01.WG_m01_C"))
  (bind _output_get (set `self.rfHud` _returnvalue))
  (`UserWidget.AddToViewport` _output_get 0)
  (`Widget.SetVisibility` _output_get "Hidden")
  (`KismetSystemLibrary.Delay` 1.0 :!label _label)
  (bind _output_get_2 (set `self.nTime` (+ (`self.nTime`) 1)))
  (`TextRenderComponent.K2_SetText` (`self.TextRender`) (`KismetTextLibrary.Conv_IntToText` _output_get_2))
  (goto _label))

(event `Key|Q`
  (params (Key :type "Key Structure"))
  (bind _returnvalue (`GameplayStatics.GetPlayerController` 0))
  (bind _rfhud (`self.rfHud`))
  (:`Pressed`
    (bind _isa (`/Engine/EditorBlueprintResources/StandardMacros.FlipFlop` :!label _label_2)
      (:`A`
        (set `PlayerController.bShowMouseCursor` _isa _returnvalue)
        (`Widget.SetVisibility` _rfhud "Visible"))
      (:`B`
        (set `PlayerController.bShowMouseCursor` _isa _returnvalue)
        (`Widget.SetVisibility` _rfhud "Hidden")))))

(event `flipVw`
  (goto _label_2))

(event `Key|E`
  (params (Key :type "Key Structure"))
  (:`Pressed`
    (set `self.nTime` 0)))

(fn `UserConstructionScript`)